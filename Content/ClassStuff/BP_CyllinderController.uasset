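; BP_CyllinderController is a test pawn that the first player controller possesses on BeginPlay, letting the player push physics cylinders.
; Pressing the JUMP input action applies a shared Force variable to Cylinder1 through Cylinder4 via AddForce, scaled by mass as AccelChange is off.
; The base Cylinder receives a zero force, so that call has no effect.
; Both BeginPlay and the jump print a debug "Hello".
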(event EventBeginPlay
  (Pawn|Possess (Game|GetPlayerController 0) self)
  (Development|PrintString "Hello"))

(event Collision|EventActorBeginOverlap
  (params (OtherActor :type Actor%20Object%20Reference)))

(event EventTick
  (params (DeltaSeconds :type Float%20%28single-precision%29)))

(event Input|ActionEvents|InputActionJUMP
  (params (Key :type Key%20Structure :default "None"))
  (bind _force (Variables|Default|GetForce))
  (:Pressed
    (Development|PrintString "Hello")
    (Physics|AddForce (Variables|Default|GetCylinder1) _force "None" false)
    (Physics|AddForce (Variables|Default|GetCylinder2) _force "None" false)
    (Physics|AddForce (Variables|Default|GetCylinder3) _force "None" false)
    (Physics|AddForce (Variables|Default|GetCylinder4) _force "None" false)
    (Physics|AddForce (Variables|Default|GetCylinder) "0, 0, 0" "None" false)))

(fn ConstructionScript)