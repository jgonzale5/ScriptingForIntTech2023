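; BP_Player is a player-controlled pawn that moves a purple ship on two axes.
; On BeginPlay, the first player controller possesses it.
; Horizontal input offsets the PurpleShipC1 component along Pawn0's negated forward vector, and Vertical input along its up vector, scaled by Speed and delta time.
; Movement changes only that component's relative location, without sweeping, so it does no collision blocking.
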(event EventBeginPlay
  (Pawn|Possess (Game|GetPlayerController 0) self))

(event Collision|EventActorBeginOverlap
  (params (OtherActor :type Actor%20Object%20Reference)))

(event EventTick
  (params (DeltaSeconds :type Float%20%28single-precision%29)))

(event Input|AxisEvents|InputAxisHorizontal
  (params (AxisValue :type Float%20%28single-precision%29))
  (Transformation|AddRelativeLocation (Variables|Default|GetPurpleShip_C_1) (* (* AxisValue (Variables|Default|GetSpeed) -1.0 (Utilities|Time|GetWorldDeltaSeconds)) (Math|Vector|GetForwardVector (Variables|Default|GetPawn_0))) false false))

(event Input|AxisEvents|InputAxisVertical
  (params (AxisValue :type Float%20%28single-precision%29))
  (Transformation|AddRelativeLocation (Variables|Default|GetPurpleShip_C_1) (* (* AxisValue (Variables|Default|GetSpeed) (Utilities|Time|GetWorldDeltaSeconds)) (Math|Vector|GetUpVector (Variables|Default|GetPawn_0))) false false))

(fn ConstructionScript)