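; BP_Balloon is a target balloon that awards points when hit by a bullet in the ship game.
; Its mesh's begin-overlap event checks the other component for a "Bullet" tag, printing debug strings, and calls PopBalloon on a match.
; PopBalloon casts the game mode to BP_ShipGame, adds the balloon's PointValue to the score and destroys the actor, so it only pops under that game mode.
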(event OnComponentBeginOverlap(StaticMeshComponent)
  (params (OverlappedComponent :type Primitive%20Component%20Object%20Reference) (OtherActor :type Actor%20Object%20Reference) (OtherComp :type Primitive%20Component%20Object%20Reference) (OtherBodyIndex :type Integer) (bFromSweep :type Boolean) (SweepResult :type Hit%20Result%20Structure%20%28by%20ref%29))
  ;[1 1 1] Purely for Debugging
  (Development|PrintString (Utilities|GetDisplayName OtherActor))
  (if (Components|ComponentHasTag OtherComp "Bullet")
    (Development|PrintString "Balloon Hit")
    (CallFunction|PopBalloon)
    (else
      (Development|PrintString "WRONG TAG"))))

(event EventBeginPlay)

(event EventTick
  (params (DeltaSeconds :type Float%20%28single-precision%29)))

(fn ConstructionScript)

(fn PopBalloon
  ;[1 1 1] When the function is called the shipgame gamemode is casted to call functions in it. This will only work if the gamemode of the level is ShipGame
  (bind _asbp_ship_game (Utilities|Casting|CastToBP_ShipGame (Game|GetGameMode)))
  ;[1 1 1] Call the AddScore function with the points value of this balloon
  (Default|AddScore _asbp_ship_game (Variables|Default|GetPointValue))
  (Actor|DestroyActor))